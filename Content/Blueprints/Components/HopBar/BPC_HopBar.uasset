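; BPC_HopBar is a component that links the owning first-person character's weapon manager to an on-screen hop bar widget.
; On BeginPlay it creates the WB_PlayerHopBar widget at a set size, adds it to the viewport and binds to the manager's weapon list change event.
; WeaponListUpdated passes all weapons to the widget to update its index, and EquipItem forwards a chosen index to the weapon manager.
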(event EventBeginPlay
  (bind _returnvalue (UserInterface|CreateWidget "/Game/Blueprints/Widgets/HopBar/WB_PlayerHopBar.WB_PlayerHopBar_C" 0 (Variables|Default|GetHop%20Bar%20Size)))
  (UserInterface|Viewport|AddtoViewport _returnvalue 0)
  (Variables|Default|SetHopBarWidget _returnvalue)
  (bind _asbp_first_person_character (Utilities|Casting|CastToBP_FirstPersonCharacter (Components|GetOwner)))
  (bind _output_get (Variables|Default|SetCharacter _asbp_first_person_character))
  (EventDispatchers|BindEventtoOnWeaponListChanged (Variables|/Script/FPS.FPSCharacter|GetWeaponManager _output_get) (EventDispatchers|CreateEvent :!event WeaponListUpdated)))

(fn WeaponListUpdated
  (Development|PrintText "??")
  (Default|UpdateIndex (Variables|Default|GetHopBarWidget) (Class|WeaponManager|GetAllWeapons (Variables|/Script/FPS.FPSCharacter|GetWeaponManager (Variables|Default|GetCharacter)))))

(fn EquipItem
  (params (Index :type Integer))
  (Class|WeaponManager|OnWeaponEquipped (Variables|/Script/FPS.FPSCharacter|GetWeaponManager (Variables|Default|GetCharacter)) Index))