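; Interaction component that lets the owning BP_FirstPersonCharacter focus and use objects it looks at.
; Each Tick it runs a short Visibility line trace from the camera and stores the first interactable hit as CurrentInteractable, sending look-at interface messages.
; That focus is cleared only when the trace hits nothing, so a direct move to another actor keeps it.
; TryInteract forwards the character to the focused actor and returns its result.
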(event EventTick
  (params (DeltaSeconds :type Float%20%28single-precision%29))
  (bind _character (Variables|Default|GetCharacter))
  (bind _returnvalue (Class|FPSCharacter|GetFirstPersonCameraComponent _character))
  (bind _returnvalue_2 (Transformation|GetWorldLocation _returnvalue))
  (Utilities|IsValid (Variables|Default|GetCharacter)
    (:Is%20Valid
      (bind (_outhit _returnvalue_3) (Collision|LineTraceByChannel _returnvalue_2 (+ _returnvalue_2 (* (Math|Vector|GetForwardVector _returnvalue) 2e+02)) "TraceTypeQuery1" false 0 "None"))
      (if _returnvalue_3
        (bind _result (Class|BPIInteraction|CanInteract(Message) (.HitActor (Collision|BreakHitResult _outhit))))
        (if _result
          (Utilities|IsValid (Variables|Default|GetCurrentInteractable)
            (:Is%20Not%20Valid
              (bind _output_get (Variables|Default|SetCurrentInteractable (.HitActor (Collision|BreakHitResult _outhit))))
              (Class|BPIInteraction|Lookat(Message) _output_get))))
        (else
          (Utilities|IsValid (Variables|Default|GetCurrentInteractable)
            (:Is%20Valid
              (Class|BPIInteraction|StopLookat(Message) (Variables|Default|GetCurrentInteractable))
              (Variables|Default|SetCurrentInteractable 0))))))))

(event EventBeginPlay
  (bind _asbp_first_person_character (Utilities|Casting|CastToBP_FirstPersonCharacter (Components|GetOwner)))
  (Variables|Default|SetCharacter _asbp_first_person_character))

(fn TryInteract
  (bind _currentinteractable (Variables|Default|GetCurrentInteractable))
  (Utilities|IsValid _currentinteractable
    (:Is%20Valid
      (bind _success (Class|BPIInteraction|Interact(Message) _currentinteractable (Variables|Default|GetCharacter)))
      (return _success))
    (:Is%20Not%20Valid
      (return false))))