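; BP_ItemPickup is an interactable world pickup that gives its item to the player's inventory.
; Looking at it shows a widget and looking away hides it.
; Interact passes the item object to the player's InventoryComponent and destroys the actor only if adding succeeds, returning the result.
; It always allows interaction and supplies a static mesh as its pickup visual, with no skeletal mesh.
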(event EventBeginPlay)

(event EventLookat
  (Rendering|SetVisibility (Variables|Default|GetWidget) true false))

(event EventStopLookat
  (Rendering|SetVisibility (Variables|Default|GetWidget) false false))

(fn ConstructionScript)

(fn CanInteract
  (return true))

(fn GetPickupSkeletalMesh
  (return 0))

(fn GetPickupStaticMesh
  (return (Variables|Default|GetStaticMesh)))

(fn Interact
  (params (Player :type BP%20First%20Person%20Character%20Object%20Reference))
  (bind _returnvalue (Class|InventoryComponent|TryAddItem (Variables|/Script/FPS.FPSCharacter|GetInventoryComponent Player) (Class|ItemActor|GetItemObject)))
  (if _returnvalue
    (Actor|DestroyActor)
    (return true)
    (else
      (return false))))