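; BP_MagazineItemObject is an inventory item object for magazines that generates its own icons from the item's actor class.
; GenerateIcons starts two asynchronous thumbnail captures with alpha and no environment, sized from the item's grid dimensions and posed using rotations from its stats.
; The second capture swaps width and height for the rotated icon, and each callback stores its texture as the default or rotated icon.
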(event EventGenerateIcons
  (bind _returnvalue (Class|ItemObject|GetItemClass))
  (bind _returnvalue_2 (Class|ItemObject|GetStats))
  (bind (_itemname _itemdescription _itemdimensions _weight _itemclass _itemactions _itemstats _itemtype _compatibleitems _maxstacksize _defaulticonrotation _rotatediconrotation) (Utilities|Struct|BreakItemStats _returnvalue_2))
  (bind _returnvalue_3 (* _itemdimensions 256.0))
  (bind _returnvalue_4 (* _itemdimensions 256.0))
  (Utilities|FlowControl|Sequence
    (:then_0
      (bind _thumbnail (|GenerateThumbnailAsync _returnvalue (Utilities|Struct|MakeThumbnailSettings (Math|Float|Truncate (.x _returnvalue_4)) (Math|Float|Truncate (.y _returnvalue_4)) true "Perspective" 1e+01 "-18.000000,-22.000000,0.000000" (Math|Transform|MakeTransform "0, 0, 0" _defaulticonrotation) "(R=0.421875,G=0.421875,B=0.421875,A=1.000000)" "0.000000,0.000000,0.000000" false) 0)
        (:then
          (bind _thumbnail_2 (|GenerateThumbnailAsync _returnvalue (Utilities|Struct|MakeThumbnailSettings (Math|Float|Truncate (.y _returnvalue_3)) (Math|Float|Truncate (.x _returnvalue_3)) true 1e+01 "0.000000,0.000000,0.000000" (Math|Transform|MakeTransform "0, 0, 0" _rotatediconrotation) false) 0)
            (:Callback
              (Class|ItemObject|SetRotatedIcon _thumbnail_2))))
        (:Callback
          (Class|ItemObject|SetDefaultIcon _thumbnail))))))