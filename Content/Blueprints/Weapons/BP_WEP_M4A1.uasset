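; Blueprint for the M4A1 weapon, an interactable pickup that adds its item object to the player's inventory.
; Weapon state changes switch visibility, collision and physics between dropped, in-hands and in-inventory, with Lookat events toggling a widget.
; Magazine events show or hide the magazine mesh and play paired load montages on weapon and first-person character meshes.
; Construction limits a scene capture component to rendering only this actor.
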(event EventReloadBP
  (Rendering|SetVisibility (Variables|Default|GetSM_Mag_A) (Class|Weapon|HasMagazine) false))

(event EventOnWeaponStateChanged
  (switch Utilities|FlowControl|Switch|SwitchonEWeaponState (Class|Weapon|GetWeaponState)
    (:Physics
      (Collision|SetCollisionEnabled (Variables|Default|GetWeaponMesh) "QueryAndPhysics")
      (Physics|SetSimulatePhysics (Variables|Default|GetWeaponMesh) true)
      (Rendering|SetActorHiddenInGame false))
    (:InHands
      (Rendering|SetActorHiddenInGame false)
      (Collision|SetCollisionEnabled (Variables|Default|GetWeaponMesh) "NoCollision"))
    (:InInventory
      (Rendering|SetActorHiddenInGame true)
      (Collision|SetCollisionEnabled (Variables|Default|GetWeaponMesh) "NoCollision"))))

(event EventStopLookat
  (Rendering|SetVisibility (Variables|Default|GetWidget) false false))

(event EventOnMagazineLoaded
  (Animation|Montage|PlayMontage (Variables|Default|GetWeaponMesh) "/Game/Art/M4A1/Anims/Weapon/A_WEP_M4A1_Load_Mag_Montage.A_WEP_M4A1_Load_Mag_Montage"
    (:then
      (Animation|Montage|PlayMontage (Class|FPSCharacter|GetMesh1P (Class|Weapon|GetCharacter)) "/Game/Art/M4A1/Anims/Character/A_CH_M4A1_Load_Mag_Montage.A_CH_M4A1_Load_Mag_Montage"))))

(event EventLookat
  (Rendering|SetVisibility (Variables|Default|GetWidget) true false))

(event EventToggleMagazine
  (params (bVisible :type Boolean))
  (Rendering|SetVisibility (Variables|Default|GetSM_Mag_A) bVisible false))

(event EventBeginPlay
  (Rendering|SetVisibility (Variables|Default|GetSM_Mag_A) false false))

(fn ConstructionScript
  (Rendering|SceneCapture|ShowOnlyActorComponents (Variables|Default|GetDefaultSceneCaptureComponent) self true))

(fn CanInteract
  (return (not (Variables|Default|GetPickedup))))

(fn Interact
  (params (Player :type BP%20First%20Person%20Character%20Object%20Reference))
  (bind _returnvalue (Class|InventoryComponent|TryAddItem (Variables|/Script/FPS.FPSCharacter|GetInventoryComponent Player) (Class|ItemActor|GetItemObject)))
  (if _returnvalue
    (return true)
    (else
      (return false))))